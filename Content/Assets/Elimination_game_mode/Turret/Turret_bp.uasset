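; Automated turret that targets and shoots at vehicles, filed under the elimination game mode.
; Each tick it picks the nearest AVS_Vehicle in sensing range with line of sight, then rotates its top toward it at constant speed with clamped pitch.
; Once the cooldown elapses and a dot product confirms aim, it fires a burst.
; A self-re-entering DoN with delays alternates projectile spawns between left and right barrel sockets.
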(event Custom|Fire
  (Variables|Private|SetTimeOfLastFire (Utilities|Time|GetGameTimeinSeconds))
  (Utilities|FlowControl|Sequence
    (:then_0
      (goto _label Reset))
    (:then_1
      (Utilities|FlowControl|DoN 5 :!label _label
        (:Exit
          (Game|SpawnActorfromClass "/Game/Assets/Elimination_game_mode/Turret/Projectile_2.Projectile_2_C" (Transformation|GetSocketTransform (Variables|Default|GetStaticMeshBarrelL) "ProjectileSocket" "RTS_World") "Undefined" 0 0)
          (Utilities|FlowControl|Delay 0.2)
          (Game|SpawnActorfromClass "/Game/Assets/Elimination_game_mode/Turret/Projectile_2.Projectile_2_C" (Transformation|GetSocketTransform (Variables|Default|GetStaticMeshBarrelR) "ProjectileSocket" "RTS_World") "Undefined" 0 0)
          (Utilities|FlowControl|Delay 0.2)
          (goto _label))))))

(event EventTick
  (params (DeltaSeconds :type Float%20%28single-precision%29))
  (Private|FindBestTarget)
  (Variables|Private|GetTarget
    (:then
      (Private|UpdateTurretRotation DeltaSeconds)
      (Private|UpdateFiring))
    (:else)))

(fn ConstructionScript)

(fn FindBestTarget
  (LocalVariables|SetBestDistance%20%28local%29 (+ (Variables|Constants|GetSensingRange) 1.0))
  (bind _outactors (Collision|SphereOverlapActors (Transformation|GetActorLocation) (Variables|Constants|GetSensingRange) (Utilities|Array|MakeArray "ObjectTypeQuery5") "/VehicleSystemPlugin/AVS_Vehicle.AVS_Vehicle_C"))
  (for _array_element _outactors
    (bind _output_get (LocalVariables|SetCurrentTarget%20%28Local%29 _array_element))
    (bind _output_get_2 (LocalVariables|SetCurrentDistance%20%28local%29 (Transformation|GetDistanceTo _output_get self)))
    (if (or (< _output_get_2 (LocalVariables|GetBestDistance%20%28local%29)) (not (Utilities|IsValid (LocalVariables|GetBestTarget%20%28local%29)))) ; Is this the closest target so far?
      (bind _result (CallFunction|HasLineOfSight (Transformation|GetWorldLocation (Variables|Default|GetStaticMeshTop)) (Transformation|GetActorLocation (LocalVariables|GetCurrentTarget%20%28Local%29)) (Utilities|Array|MakeArray self (LocalVariables|GetCurrentTarget%20%28Local%29))))
      (if _result
        (LocalVariables|SetBestTarget%20%28local%29 (LocalVariables|GetCurrentTarget%20%28Local%29))
        (LocalVariables|SetBestDistance%20%28local%29 (LocalVariables|GetCurrentDistance%20%28local%29)))))
  (Variables|Private|SetTarget (LocalVariables|GetBestTarget%20%28local%29)))

(fn UpdateTurretRotation
  (params (Delta%20secs :type Float%20%28single-precision%29))
  (bind _output_get (LocalVariables|SetNewRotation (Class|KismetMathLibrary|RInterptoConstant (Transformation|GetWorldRotation (Variables|Default|GetStaticMeshTop)) (Math|Rotator|FindLookatRotation (Transformation|GetWorldLocation (Variables|Default|GetStaticMeshTop)) (Transformation|GetActorLocation (Variables|Private|GetTarget))) Delta%20secs (Variables|Constants|GetRotation%20Speed))))
  (Transformation|SetWorldRotation (Variables|Default|GetStaticMeshTop) (Math|Rotator|MakeRotator (.roll _output_get) (Math|Float|ClampAngle (.pitch _output_get) -45.0 75.0) (.yaw _output_get)) false false))

(fn UpdateFiring
  (if (> (- (Utilities|Time|GetGameTimeinSeconds) (Variables|Private|GetTimeOfLastFire)) (Variables|Constants|GetRateOfFire)) ; Has rate of fire cooled down
    (if (> (Math|Vector|DotProduct (Math|Vector|GetUnitDirection(Vector) (Transformation|GetWorldLocation (Variables|Default|GetStaticMeshTop)) (Transformation|GetActorLocation (Variables|Private|GetTarget))) (Math|Vector|GetForwardVector (Variables|Default|GetStaticMeshTop))) 0.99) ; Is Turret Facing Target??
      (CallFunction|Fire))))