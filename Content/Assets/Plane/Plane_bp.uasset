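; Plane actor that flies along a spline path, starting at BeginPlay.
; It finds a Plane_spline actor in the level and plays the MovePlaneT timeline, with play rate set to the inverse of TimeToComplete.
; Each update maps the timeline's track to a distance along the spline, then sets the actor's transform from the world-space location and local-space rotation there.
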(event Custom|Move%20Object
  (bind _spline_ref (Variables|Default|Getspline%20ref))
  (bind _plane_spline (Variables|/Game/Assets/Plane/Plane_spline.Plane_spline_C|Getplane_Spline _spline_ref))
  (Components|Timeline|SetPlayRate (Variables|Default|GetMove%20plane%20t) (/ 1.0 (Variables|Default|GetTime%20to%20complete)))
  (bind _move_track (Timeline|Move%20plane%20t Play)
    (:Update
      (Transformation|SetActorTransform (Math|Transform|MakeTransform (Spline|GetLocationatDistanceAlongSpline _plane_spline (Math|Float|Lerp 0.0 (Spline|GetSplineLength (Variables|/Game/Assets/Plane/Plane_spline.Plane_spline_C|Getplane_Spline (Variables|Default|Getspline%20ref))) _move_track) "World") (Spline|GetRotationatDistanceAlongSpline _plane_spline (Math|Float|Lerp 0.0 (Spline|GetSplineLength (Variables|/Game/Assets/Plane/Plane_spline.Plane_spline_C|Getplane_Spline (Variables|Default|Getspline%20ref))) _move_track) "Local") "1,1,1")))))

(event EventBeginPlay
  (bind _returnvalue (Actor|GetActorOfClass "/Game/Assets/Plane/Plane_spline.Plane_spline_C"))
  (Variables|Default|Setspline%20ref _returnvalue)
  (CallFunction|MoveObject))

(fn ConstructionScript)