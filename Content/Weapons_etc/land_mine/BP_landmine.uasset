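; Landmine actor that applies damage to any Delorean_AVS vehicle each time one overlaps it.
; A DoOnce limits the explosion emitter, sound and controller rumble to one trigger, centered on the player's vehicle rather than the mine.
; It also pitches the player's mesh by 10 degrees and raises CustomEventPlaying for one second.
; The closing rotation call reapplies the current rotation, so it does not undo the tilt.
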(event EventBeginPlay)

(event Collision|EventActorBeginOverlap
  (params (OtherActor :type Actor%20Object%20Reference))
  (bind _asdelorean_avs (Utilities|Casting|CastToDelorean_AVS OtherActor))
  (Game|Damage|ApplyDamage _asdelorean_avs 25.0 0 0)
  (bind _asdelorean_avs_2 (Utilities|Casting|CastToDelorean_AVS (Game|Player|GetPlayerPawn 0)))
  (Utilities|FlowControl|DoOnce false
    (:Completed
      (Effects|SpawnEmitteratLocation "/Game/Realistic_Starter_VFX_Pack_Vol2/Particles/Explosion/P_Explosion_Big_A.P_Explosion_Big_A" (Transformation|GetWorldLocation (Default|GetVehicleMesh _asdelorean_avs_2)) "0, 0, 0" "3.000000,3.000000,3.000000")
      (Audio|PlaySoundatLocation "/Game/Sounds/explosion.explosion" (Transformation|GetWorldLocation (Default|GetVehicleMesh _asdelorean_avs_2)) "0, 0, 0" 1.0 1.0 0.0 0 0 0)
      (Game|Feedback|PlayDynamicForceFeedback (Game|GetPlayerController 0) 1.0 1.0 true true true true)
      (bind _asdelorean_avs_3 (Utilities|Casting|CastToDelorean_AVS (Game|Player|GetPlayerPawn 0)))
      (Variables|/Game/AVS/AVS_Master.AVS_Master_C|Setcustom%20event%20playing? _asdelorean_avs_3 true)
      (Transformation|SetWorldRotation (Variables|/Script/VehicleSystemPlugin.VehicleSystemBase|GetVehicleMesh _asdelorean_avs_3) (Math|Rotator|MakeRotator (.roll (Transformation|GetWorldRotation (Variables|/Script/VehicleSystemPlugin.VehicleSystemBase|GetVehicleMesh _asdelorean_avs_3))) (+ (.pitch (Transformation|GetWorldRotation (Variables|/Script/VehicleSystemPlugin.VehicleSystemBase|GetVehicleMesh _asdelorean_avs_3))) 1e+01) (.yaw (Transformation|GetWorldRotation (Variables|/Script/VehicleSystemPlugin.VehicleSystemBase|GetVehicleMesh _asdelorean_avs_3)))) false false)
      (Utilities|FlowControl|Delay 1.0)
      (Transformation|SetWorldRotation (Variables|/Script/VehicleSystemPlugin.VehicleSystemBase|GetVehicleMesh _asdelorean_avs_3) (Math|Rotator|MakeRotator (.roll (Transformation|GetWorldRotation (Variables|/Script/VehicleSystemPlugin.VehicleSystemBase|GetVehicleMesh _asdelorean_avs_3))) (.pitch (Transformation|GetWorldRotation (Variables|/Script/VehicleSystemPlugin.VehicleSystemBase|GetVehicleMesh _asdelorean_avs_3))) (.yaw (Transformation|GetWorldRotation (Variables|/Script/VehicleSystemPlugin.VehicleSystemBase|GetVehicleMesh _asdelorean_avs_3)))) false false)
      (Variables|/Game/AVS/AVS_Master.AVS_Master_C|Setcustom%20event%20playing? _asdelorean_avs_3 false))))

(event EventTick
  (params (DeltaSeconds :type Float%20%28single-precision%29)))

(fn ConstructionScript)