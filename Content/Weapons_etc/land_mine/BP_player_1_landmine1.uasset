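; Player 1's landmine actor, which damages AI cars 2, 3 and 4 when they overlap it.
; A chain of casts identifies the car, applies LandmineDamage, then spawns a scaled-up explosion at the car's location and destroys the mine.
; Each car branch has a DoOnce guarding the explosion, with a delayed reset placed after DestroyActor.
; Other overlapping actors are ignored.
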(event EventBeginPlay)

(event Collision|EventActorBeginOverlap
  (params (OtherActor :type Actor%20Object%20Reference))
  (bind _asbp_ai_car_2 (Utilities|Casting|CastToBP_ai_car_2 OtherActor)
    (:then
      (Game|Damage|ApplyDamage _asbp_ai_car_2 (Variables|Default|Getlandmine%20damage) 0 0)
      (Utilities|FlowControl|DoOnce false :!label _label
        (:Completed
          (Effects|SpawnEmitteratLocation "/Game/Realistic_Starter_VFX_Pack_Vol2/Particles/Explosion/P_Explosion_Big_A.P_Explosion_Big_A" (Transformation|GetWorldLocation (Variables|/Script/Engine.Actor|GetRootComponent _asbp_ai_car_2)) "0, 0, 0" "3.000000,3.000000,3.000000")
          (Actor|DestroyActor)
          (Utilities|FlowControl|Delay 5.0)
          (goto _label Reset))))
    (:CastFailed
      (bind _asbp_ai_car_3 (Utilities|Casting|CastToBP_ai_car_3 OtherActor)
        (:then
          (Game|Damage|ApplyDamage _asbp_ai_car_3 (Variables|Default|Getlandmine%20damage) 0 0)
          (Utilities|FlowControl|DoOnce false :!label _label_2
            (:Completed
              (Effects|SpawnEmitteratLocation "/Game/Realistic_Starter_VFX_Pack_Vol2/Particles/Explosion/P_Explosion_Big_A.P_Explosion_Big_A" (Transformation|GetWorldLocation (Variables|/Script/Engine.Actor|GetRootComponent _asbp_ai_car_3)) "0, 0, 0" "3.000000,3.000000,3.000000")
              (Actor|DestroyActor)
              (Utilities|FlowControl|Delay 5.0)
              (goto _label_2 Reset))))
        (:CastFailed
          (bind _asbp_ai_car_4 (Utilities|Casting|CastToBP_ai_car_4 OtherActor))
          (Game|Damage|ApplyDamage _asbp_ai_car_4 (Variables|Default|Getlandmine%20damage) 0 0)
          (Utilities|FlowControl|DoOnce false :!label _label_3
            (:Completed
              (Effects|SpawnEmitteratLocation "/Game/Realistic_Starter_VFX_Pack_Vol2/Particles/Explosion/P_Explosion_Big_A.P_Explosion_Big_A" (Transformation|GetWorldLocation (Variables|/Script/Engine.Actor|GetRootComponent _asbp_ai_car_4)) "0, 0, 0" "3.000000,3.000000,3.000000")
              (Actor|DestroyActor)
              (Utilities|FlowControl|Delay 5.0)
              (goto _label_3 Reset))))))))

(event EventTick
  (params (DeltaSeconds :type Float%20%28single-precision%29)))

(fn ConstructionScript)