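; Homing rocket launcher projectile that seeks the nearest actor tagged "Homing" and explodes on overlap.
; From BeginPlay, a delay loop repeatedly runs FindHomingTarget, a linear distance search over tagged actors, and feeds the result to ProjectileMovement as its homing component.
; Any overlap damages the stored HomingTarget rather than the overlapped actor, plays explosion effect and sound at that target's location, and destroys the rocket.
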(event Custom|lock%20on%20target
  (bind _projectilemovement (Variables|Default|GetProjectileMovement))
  ;[1 1 1] find nearest target with tag 'Homing'
  (bind _homing_target (CallFunction|FindHomingTarget))
  (Variables|/Script/Engine.ProjectileMovementComponent|SetHomingTargetComponent _projectilemovement _homing_target)
  (Variables|/Script/Engine.ProjectileMovementComponent|SetbIsHomingProjectile _projectilemovement true))

(event EventBeginPlay
  ;[1 1 1] find nearest target (loop)
  (CallFunction|LockonTarget :!label _label)
  (Utilities|FlowControl|Delay 0.5)
  (goto _label))

(event Collision|EventActorBeginOverlap
  (params (OtherActor :type Actor%20Object%20Reference))
  (bind _homing_target (Variables|Default|GetHoming%20target))
  (bind _returnvalue (Transformation|GetActorLocation _homing_target))
  (Game|Damage|ApplyDamage _homing_target 3e+01 0 0)
  (Effects|SpawnEmitteratLocation "/Game/Realistic_Starter_VFX_Pack_Vol2/Particles/Explosion/P_Explosion_Big_A.P_Explosion_Big_A" _returnvalue)
  (Actor|DestroyActor)
  (Audio|PlaySoundatLocation "/Game/StarterContent/Audio/Explosion02.Explosion02" _returnvalue "0, 0, 0" 1.0 1.0 0.0 0 0 0))

(fn ConstructionScript)

(fn FindHomingTarget
  (bind _outactors (Actor|GetAllActorsOfClasswithTag "/Script/Engine.Actor" "Homing"))
  (for _array_element _outactors
    (if (< (Math|Vector|VectorLength (- (Transformation|GetActorLocation _array_element) (Transformation|GetActorLocation))) (Variables|Default|Getclosest%20distance))
      (Variables|Default|Setclosest%20distance (Math|Vector|VectorLength (- (Transformation|GetActorLocation _array_element) (Transformation|GetActorLocation))))
      (Variables|Default|SetHoming%20target _array_element)))
  (return (Actor|GetComponentbyClass (Variables|Default|GetHoming%20target) "/Script/Engine.SceneComponent")))