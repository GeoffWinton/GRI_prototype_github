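; Test player car with a timed turbo boost, mounted minigun and adjustable chase camera, skinned with a material from the game instance.
; Boost overrides mesh velocity along the forward vector, then resets it after a delay.
; Holding fire shows the gun effect, plays sound and loops a timer-driven line trace that applies damage and impact emitters.
; Axis inputs interpolate spring-arm zoom and yaw; incoming damage sets HitPoints to damage minus current HitPoints.
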(event EventBeginPlay
  (bind _asbp_gameinstance_mats (Utilities|Casting|CastTo (Game|GetGameInstance)))
  (Rendering|Material|SetMaterial (Variables|Default|GetVehicleMesh) 0 (Variables|Default|Getmaterial_change _asbp_gameinstance_mats))
  (Development|PrintString 0 (Utilities|GetDisplayName 0) true true "(R=0.000000,G=0.660000,B=1.000000,A=1.000000)" 3e+01))

(event Collision|EventActorBeginOverlap
  (params (OtherActor :type Actor%20Object%20Reference)))

(event Game|Damage|EventAnyDamage
  (params (Damage :type Float%20%28single-precision%29) (DamageType :type Damage%20Type%20Object%20Reference) (InstigatedBy :type Controller%20Object%20Reference) (DamageCauser :type Actor%20Object%20Reference))
  (Variables|Default|Sethit%20points (Math|Float|Truncate (- Damage (Math|Conversions|ToFloat(Integer) (Variables|Default|Gethit%20points))))))

(event Input|ActionEvents|InputActionturboboost
  (params (Key :type Key%20Structure :default "None"))
  ;[1 1 1] turbo boost
  (:Pressed
    (if (not (Variables|Default|Getturbobooston))
      (bind _output_get (Variables|Default|Setpreboost%20vector (Transformation|GetActorForwardVector)))
      (Physics|SetPhysicsLinearVelocity (Variables|Default|GetVehicleMesh) (* _output_get 2e+04) false "None")
      (Variables|Default|Setturbobooston true)
      (Utilities|FlowControl|Delay 0 (Variables|Default|Getboost%20length))
      (Physics|SetPhysicsLinearVelocity (Variables|Default|GetVehicleMesh) (Variables|Default|Getpreboost%20vector) false "None")
      (Variables|Default|Setturbobooston false))))

(event Input|ActionEvents|InputActionfiregun
  (params (Key :type Key%20Structure :default "None"))
  ;[1 1 1] gunfire
  (:Pressed
    (Rendering|SetVisibility (Variables|Default|GetP_AssaultRifle_MF) true false)
    (bind _returnvalue (Audio|SpawnSound2D 0 0 1.0 1.0 0.0 0))
    (Variables|Default|Setgunfire _returnvalue)
    (CallFunction|WeaponTrace)
    (Utilities|Time|SetTimerbyFunctionName 0 "weapon trace" (Variables|Default|Getweapon%20fire%20rate) true))
  (:Released
    (Rendering|SetVisibility (Variables|Default|GetP_AssaultRifle_MF) false false)
    (Audio|Components|Audio|Stop (Variables|Default|Getgunfire))
    (Audio|PlaySoundatLocation 0 0 (Variables|/Script/Engine.SceneComponent|GetRelativeLocation (Variables|Default|Getmini_gun)) "0, 0, 0" 0.7 1.0 0.0 0 0 0)
    (Utilities|Time|ClearTimerbyFunctionName 0 "weapon trace")))

(event Input|AxisEvents|InputAxiscamerazoom
  (params (AxisValue :type Float%20%28single-precision%29))
  ;[1 1 1] camera zoom
  (bind _output_get (Variables|Default|Setspring%20arm%20target (Math|Float|Clamp(Float) (+ (* AxisValue 1e+01) (Variables|Default|Getspring%20arm%20target)) 3e+02 3e+03)))
  (Variables|/Script/Engine.SpringArmComponent|SetTargetArmLength (Variables|Default|GetSpringArm) (Math|Interpolation|FInterpTo (Variables|/Script/Engine.SpringArmComponent|GetTargetArmLength (Variables|Default|GetSpringArm)) _output_get (Utilities|Time|GetWorldDeltaSeconds) 1e+01)))

(event Input|AxisEvents|InputAxiscamerarotate
  (params (AxisValue :type Float%20%28single-precision%29))
  ;[1 1 1] camera rotation
  (if (!= AxisValue 0.0)
    (bind _output_get (Variables|Default|Setspring%20arm%20rotation (Math|Vector|MakeVector 0.0 0.0 (.yaw (Math|Rotator|MakeRotator 0.0 0.0 (Math|Float|Clamp(Float) (+ (* AxisValue 5.0) (.z (Variables|Default|Getspring%20arm%20rotation))) -9e+01 9e+01))))))
    (Transformation|SetRelativeRotation (Variables|Default|GetSpringArm) (Math|Rotator|MakeRotator 0.0 -2e+01 (Math|Interpolation|FInterpTo (.yaw (Variables|/Script/Engine.SceneComponent|GetRelativeRotation (Variables|Default|GetSpringArm))) (.z _output_get) (Utilities|Time|GetWorldDeltaSeconds) 1e+01)) false false)
    (else
      (bind _output_get_2 (Variables|Default|Setspring%20arm%20rotation "0,-20.000000, 0"))
      (Transformation|SetRelativeRotation (Variables|Default|GetSpringArm) (Math|Rotator|MakeRotator 0.0 -2e+01 (Math|Interpolation|FInterpTo (.yaw (Variables|/Script/Engine.SceneComponent|GetRelativeRotation (Variables|Default|GetSpringArm))) (.z _output_get_2) (Utilities|Time|GetWorldDeltaSeconds) 1e+01)) false false))))

(fn ConstructionScript)

(fn WeaponTrace
  (bind _arrow (Variables|Default|GetArrow))
  (bind _returnvalue (Transformation|GetWorldLocation _arrow))
  ;[1 1 1] gunfire
  (bind _outhit (Collision|LineTraceByChannel 0 _returnvalue (+ _returnvalue (* (Math|Vector|GetForwardVector (Transformation|GetWorldRotation _arrow)) (Variables|Default|Getweapon%20range))) "TraceTypeQuery1" false 0 "None"))
  (if (.bBlockingHit (Collision|BreakHitResult _outhit))
    (Game|Damage|ApplyDamage (.HitActor (Collision|BreakHitResult _outhit)) 1e+01 0 0)
    (Effects|SpawnEmitteratLocation 0 0 (.Location (Collision|BreakHitResult _outhit)) "0, 0, 0" "3.000000,3.000000,3.000000")))