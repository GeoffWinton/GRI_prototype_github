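; AI-driven car that follows the racing line of a BP_AI_spline_line and manages its own speed.
; Each tick it steers toward a speed-scaled look-ahead point on the first spline found.
; It accelerates under a base speed limit; above it, a forward trace hit triggers either distance-mapped braking or, inside CornerIndex actors, corner-specific limits.
; Only slight-right and hairpin-left corners are handled; debug trace and brake printout remain active.
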(event EventBeginPlay
  (|CallParentFunction)
  (CallFunction|StartEngine)
  (CallFunction|SetHandbrakeInput false)
  (CallFunction|SetShifterPosition "NewEnumerator3"))

(event Collision|EventActorBeginOverlap
  (params (OtherActor :type Actor%20Object%20Reference)))

(event EventTick
  (params (DeltaSeconds :type Float%20%28single-precision%29))
  (bind _outactors (Actor|GetAllActorsOfClass "/Game/Geoff_migrated_assets/car_meshes/AI_Car/BP_AI_spline_line.BP_AI_spline_line_C"))
  (bind _returnvalue (CallFunction|GetLane _outactors))
  (CallFunction|SetSteeringInput _returnvalue)
  (Utilities|SpeedLimiter 1e+01
    (:under%20speed%20limit
      (CallFunction|Setinput 1.0 0.0))
    (:over%20speed%20limit
      (CallFunction|LineTracer)
      (if (Variables|Default|GetFrontLineTraceHit?)
        (bind _corner (Utilities|GetCorner)
          (:IsInCorner
            (bind _ascorner_index (Utilities|Casting|CastToCornerIndex _corner))
            (switch Utilities|FlowControl|Switch|SwitchonE_Turnindex (Variables|/Game/Geoff_migrated_assets/car_meshes/AI_Car/CornerIndex.CornerIndex_C|GetTurnIndex _ascorner_index)
              (:NewEnumerator0
                (Utilities|SpeedLimiter 1e+01
                  (:under%20speed%20limit
                    (CallFunction|Setinput 0.75 0.0))
                  (:over%20speed%20limit
                    (CallFunction|Setinput 0.0 1.0))))
              (:NewEnumerator1
                (Utilities|SpeedLimiter 5.0
                  (:under%20speed%20limit
                    (CallFunction|Setinput 0.75 0.0))
                  (:over%20speed%20limit
                    (CallFunction|Setinput 0.0 1.0))))))
          (:NotInCorner
            (CallFunction|Setinput 0.0 (Math|Float|MapRangeClamped (.distance (Variables|Default|GetFrontLineTraceHitResult)) 0.0 1.0 0.0 2.5e+03))))
        (else
          (CallFunction|Setinput 0.75 0.0))))))

(fn ConstructionScript
  (|CallParentFunction))

(fn GetLane
  (params (splines :type Array%20of%20BP%20AI%20Spline%20Line%20Object%20References))
  (bind _returnvalue (Transformation|GetActorLocation))
  (bind _output (Utilities|Array|Get(acopy) splines))
  (return (Math|Float|MapRangeUnclamped (.yaw (Math|Rotator|Delta(Rotator) (Math|Rotator|FindLookatRotation _returnvalue (Spline|FindLocationClosesttoWorldLocation (Variables|/Game/Geoff_migrated_assets/car_meshes/AI_Car/BP_AI_spline_line.BP_AI_spline_line_C|GetRacing_line_AI _output) (+ (* (Math|Vector|Normalize (Class|SplineComponent|FindTangentClosesttoWorldLocation (Variables|/Game/Geoff_migrated_assets/car_meshes/AI_Car/BP_AI_spline_line.BP_AI_spline_line_C|GetRacing_line_AI _output) _returnvalue "World")) (Math|Float|MapRangeClamped (CallFunction|GetAirSpeed) 0.0 8e+01 1e+02 1e+03)) _returnvalue) "World")) (Transformation|GetActorRotation))) -9e+01 9e+01 -0.25 0.25)))

(fn Setinput
  (params (Throttle :type Float%20%28single-precision%29) (Brake :type Float%20%28single-precision%29))
  (CallFunction|SetThrottleInput Throttle)
  (CallFunction|SetBrakeInput Brake)
  (Development|PrintString (Utilities|String|ToString(Boolean) (CallFunction|GetBrakeApplied))))

(fn LineTracer
  (bind _line_trace_start (Variables|Default|Getline%20trace%20start))
  (bind _returnvalue (Transformation|GetWorldLocation _line_trace_start))
  (bind (_outhit _returnvalue_2) (Collision|LineTraceByChannel _returnvalue (+ _returnvalue (* (Math|Vector|GetForwardVector _line_trace_start) 2.5e+03)) "TraceTypeQuery1" false 0 "ForDuration"))
  (Variables|Default|SetFrontLineTraceHitResult _outhit)
  (Variables|Default|SetFrontLineTraceHit? _returnvalue_2))