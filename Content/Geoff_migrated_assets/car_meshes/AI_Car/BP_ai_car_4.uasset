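; AI opponent car 4 for a combat race: drives itself, shoots, drops landmines and takes damage.
; A timeline moves it along BP_ai_spline_car4 at periodically randomized speed, with ground traces setting height and pitch.
; Tick publishes its transform to AVS_GameMode as car 3, fires trace weapons and pauses behind cars 2 and 3.
; Damage reveals fire and smoke; death means elimination (flagged as car 1) or a flashing respawn.
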(event Custom|visible%20damage_aicar2
  ;[1 1 1] damage visibility
  (if (>= (/ (Variables|Default|GetAI_car2_hitpoints) (Variables|Default|GetAI_car2_maxhitpoints)) 0.75)
    (Rendering|SetVisibility (Variables|Default|Getai_car_2_smoke) false false))
  (if (< (/ (Variables|Default|GetAI_car2_hitpoints) (Variables|Default|GetAI_car2_maxhitpoints)) 0.75)
    (Rendering|SetVisibility (Variables|Default|Getai_car2_front_fire) true false)
    (if (< (/ (Variables|Default|GetAI_car2_hitpoints) (Variables|Default|GetAI_car2_maxhitpoints)) 0.5)
      (Rendering|SetVisibility (Variables|Default|Getai_car2_rear_fire) true false)
      (if (< (/ (Variables|Default|GetAI_car2_hitpoints) (Variables|Default|GetAI_car2_maxhitpoints)) 0.25)
        (Rendering|SetVisibility (Variables|Default|Getai_car_2_smoke) true false)))))

(event Custom|move%20ai%20car
  (bind _returnvalue (Transformation|GetActorRotation))
  (bind _front_pitch_trace_start (Variables|Default|Getfront%20pitch%20trace%20start))
  (bind _height_trace_start (Variables|Default|Getheight%20trace%20start))
  (bind _rear_pitch_trace_start (Variables|Default|Getrear%20pitch%20trace%20start))
  (bind _right_roll_trace_start1 (Variables|Default|Getright%20roll%20trace%20start1))
  (bind _left_roll_trace_start2 (Variables|Default|Getleft%20roll%20trace%20start2))
  (bind _returnvalue_2 (Transformation|GetWorldLocation _front_pitch_trace_start))
  (bind _returnvalue_3 (Transformation|GetWorldLocation _rear_pitch_trace_start))
  (bind _returnvalue_4 (Transformation|GetWorldLocation _height_trace_start))
  (bind _returnvalue_5 (Transformation|GetWorldLocation _right_roll_trace_start1))
  (bind _returnvalue_6 (Transformation|GetWorldLocation _left_roll_trace_start2))
  (Components|Timeline|SetPlayRate (Variables|Default|Getmove%20ai%20car) (/ 1.0 (Variables|Default|Gettime%20to%20complete%20%28seconds%29)))
  (bind _newtrack_0 (Timeline|move%20ai%20car Play)
    (:Update
      (bind _outhit (Collision|LineTraceByChannel _returnvalue_4 (+ _returnvalue_4 (* (Math|Vector|GetForwardVector (Transformation|GetWorldRotation _height_trace_start)) 1e+03)) "TraceTypeQuery1" false 0 "None"))
      (bind _outhit_2 (Collision|LineTraceByChannel _returnvalue_5 (+ _returnvalue_5 (* (Math|Vector|GetForwardVector (Transformation|GetWorldRotation _right_roll_trace_start1)) 1e+03)) "TraceTypeQuery1" false 0 "None"))
      (bind _outhit_3 (Collision|LineTraceByChannel _returnvalue_6 (+ _returnvalue_6 (* (Math|Vector|GetForwardVector (Transformation|GetWorldRotation _left_roll_trace_start2)) 1e+03)) "TraceTypeQuery1" false 0 "None"))
      (bind _outhit_4 (Collision|LineTraceByChannel _returnvalue_2 (+ _returnvalue_2 (* (Math|Vector|GetForwardVector (Transformation|GetWorldRotation _front_pitch_trace_start)) 1e+03)) "TraceTypeQuery1" false 0 "None"))
      (bind _outhit_5 (Collision|LineTraceByChannel _returnvalue_3 (+ _returnvalue_3 (* (Math|Vector|GetForwardVector (Transformation|GetWorldRotation _rear_pitch_trace_start)) 1e+03)) "TraceTypeQuery1" false 0 "None"))
      (if (< (.Distance (Collision|BreakHitResult _outhit_4)) (.Distance (Collision|BreakHitResult _outhit_5)))
        (Variables|Default|SetReturn%20Value%20Y%20%28Pitch%29 (+ (.pitch _returnvalue) 0.1))
        (else
          (Variables|Default|SetReturn%20Value%20Y%20%28Pitch%29 (- (.pitch _returnvalue) 0.1))))
      (Transformation|SetActorTransform (Math|Transform|MakeTransform (Math|Vector|MakeVector (.x (Spline|GetLocationatDistanceAlongSpline (Variables|/Game/Geoff_migrated_assets/car_meshes/AI_Car/BP_ai_spline_car4.BP_ai_spline_car4_C|GetSpline (Variables|Default|Getspline2%20ref)) (Math|Float|Lerp 0.0 (Spline|GetSplineLength (Variables|/Game/Geoff_migrated_assets/car_meshes/AI_Car/BP_ai_spline_car4.BP_ai_spline_car4_C|GetSpline (Variables|Default|Getspline2%20ref))) _newtrack_0) "World")) (.y (Spline|GetLocationatDistanceAlongSpline (Variables|/Game/Geoff_migrated_assets/car_meshes/AI_Car/BP_ai_spline_car4.BP_ai_spline_car4_C|GetSpline (Variables|Default|Getspline2%20ref)) (Math|Float|Lerp 0.0 (Spline|GetSplineLength (Variables|/Game/Geoff_migrated_assets/car_meshes/AI_Car/BP_ai_spline_car4.BP_ai_spline_car4_C|GetSpline (Variables|Default|Getspline2%20ref))) _newtrack_0) "World")) (+ (- (.z (Transformation|GetActorLocation)) (.Distance (Collision|BreakHitResult _outhit))) 125.0)) (Math|Rotator|MakeRotator (Variables|Default|GetReturn%20Value%20X%20%28Roll%29) (Variables|Default|GetReturn%20Value%20Y%20%28Pitch%29) (.yaw (Spline|GetRotationatDistanceAlongSpline (Variables|/Game/Geoff_migrated_assets/car_meshes/AI_Car/BP_ai_spline_car4.BP_ai_spline_car4_C|GetSpline (Variables|Default|Getspline2%20ref)) (Math|Float|Lerp 0.0 (Spline|GetSplineLength (Variables|/Game/Geoff_migrated_assets/car_meshes/AI_Car/BP_ai_spline_car4.BP_ai_spline_car4_C|GetSpline (Variables|Default|Getspline2%20ref))) _newtrack_0) "World"))) "1,1,1")))))

(event Custom|change%20AI%20car%20speed
  (bind _returnvalue (Transformation|GetActorRotation))
  (bind _front_pitch_trace_start (Variables|Default|Getfront%20pitch%20trace%20start))
  (bind _height_trace_start (Variables|Default|Getheight%20trace%20start))
  (bind _rear_pitch_trace_start (Variables|Default|Getrear%20pitch%20trace%20start))
  (bind _right_roll_trace_start1 (Variables|Default|Getright%20roll%20trace%20start1))
  (bind _left_roll_trace_start2 (Variables|Default|Getleft%20roll%20trace%20start2))
  (bind _returnvalue_2 (Transformation|GetWorldLocation _front_pitch_trace_start))
  (bind _returnvalue_3 (Transformation|GetWorldLocation _rear_pitch_trace_start))
  (bind _returnvalue_4 (Transformation|GetWorldLocation _height_trace_start))
  (bind _returnvalue_5 (Transformation|GetWorldLocation _right_roll_trace_start1))
  (bind _returnvalue_6 (Transformation|GetWorldLocation _left_roll_trace_start2))
  (Components|Timeline|SetPlayRate (Variables|Default|Getmove%20ai%20car) (* (/ 1.0 (Variables|Default|Gettime%20to%20complete%20%28seconds%29)) (Math|Random|RandomFloatinRange 0.7 1.3)))
  (bind _newtrack_0 (Timeline|move%20ai%20car Play)
    (:Update
      (bind _outhit (Collision|LineTraceByChannel _returnvalue_4 (+ _returnvalue_4 (* (Math|Vector|GetForwardVector (Transformation|GetWorldRotation _height_trace_start)) 1e+03)) "TraceTypeQuery1" false 0 "None"))
      (bind _outhit_2 (Collision|LineTraceByChannel _returnvalue_5 (+ _returnvalue_5 (* (Math|Vector|GetForwardVector (Transformation|GetWorldRotation _right_roll_trace_start1)) 1e+03)) "TraceTypeQuery1" false 0 "None"))
      (bind _outhit_3 (Collision|LineTraceByChannel _returnvalue_6 (+ _returnvalue_6 (* (Math|Vector|GetForwardVector (Transformation|GetWorldRotation _left_roll_trace_start2)) 1e+03)) "TraceTypeQuery1" false 0 "None"))
      (bind _outhit_4 (Collision|LineTraceByChannel _returnvalue_2 (+ _returnvalue_2 (* (Math|Vector|GetForwardVector (Transformation|GetWorldRotation _front_pitch_trace_start)) 1e+03)) "TraceTypeQuery1" false 0 "None"))
      (bind _outhit_5 (Collision|LineTraceByChannel _returnvalue_3 (+ _returnvalue_3 (* (Math|Vector|GetForwardVector (Transformation|GetWorldRotation _rear_pitch_trace_start)) 1e+03)) "TraceTypeQuery1" false 0 "None"))
      (if (< (.Distance (Collision|BreakHitResult _outhit_4)) (.Distance (Collision|BreakHitResult _outhit_5)))
        (Variables|Default|SetReturn%20Value%20Y%20%28Pitch%29 (+ (.pitch _returnvalue) 0.1))
        (else
          (Variables|Default|SetReturn%20Value%20Y%20%28Pitch%29 (- (.pitch _returnvalue) 0.1))))
      (Transformation|SetActorTransform (Math|Transform|MakeTransform (Math|Vector|MakeVector (.x (Spline|GetLocationatDistanceAlongSpline (Variables|/Game/Geoff_migrated_assets/car_meshes/AI_Car/BP_ai_spline_car4.BP_ai_spline_car4_C|GetSpline (Variables|Default|Getspline2%20ref)) (Math|Float|Lerp 0.0 (Spline|GetSplineLength (Variables|/Game/Geoff_migrated_assets/car_meshes/AI_Car/BP_ai_spline_car4.BP_ai_spline_car4_C|GetSpline (Variables|Default|Getspline2%20ref))) _newtrack_0) "World")) (.y (Spline|GetLocationatDistanceAlongSpline (Variables|/Game/Geoff_migrated_assets/car_meshes/AI_Car/BP_ai_spline_car4.BP_ai_spline_car4_C|GetSpline (Variables|Default|Getspline2%20ref)) (Math|Float|Lerp 0.0 (Spline|GetSplineLength (Variables|/Game/Geoff_migrated_assets/car_meshes/AI_Car/BP_ai_spline_car4.BP_ai_spline_car4_C|GetSpline (Variables|Default|Getspline2%20ref))) _newtrack_0) "World")) (+ (- (.z (Transformation|GetActorLocation)) (.Distance (Collision|BreakHitResult _outhit))) 125.0)) (Math|Rotator|MakeRotator (Variables|Default|GetReturn%20Value%20X%20%28Roll%29) (Variables|Default|GetReturn%20Value%20Y%20%28Pitch%29) (.yaw (Spline|GetRotationatDistanceAlongSpline (Variables|/Game/Geoff_migrated_assets/car_meshes/AI_Car/BP_ai_spline_car4.BP_ai_spline_car4_C|GetSpline (Variables|Default|Getspline2%20ref)) (Math|Float|Lerp 0.0 (Spline|GetSplineLength (Variables|/Game/Geoff_migrated_assets/car_meshes/AI_Car/BP_ai_spline_car4.BP_ai_spline_car4_C|GetSpline (Variables|Default|Getspline2%20ref))) _newtrack_0) "World"))) "1,1,1")))))

(event EventBeginPlay
  (bind _asbp_gameinstance_mats (Utilities|Casting|CastToBP_gameinstance_mats (Game|GetGameInstance)))
  (if (Variables|/Game/Geoff_migrated_assets/Garage_stuff/BP_gameinstance_mats.BP_gameinstance_mats_C|Getelimination%20race? _asbp_gameinstance_mats)
    (Variables|Default|Setelimination%20race? true)
    (Variables|Default|Settime%20to%20complete%20%28seconds%29 6e+01))
  (bind _asbp_gameinstance_mats_2 (Utilities|Casting|CastToBP_gameinstance_mats (Game|GetGameInstance)))
  (Variables|Default|Setlaps%20left (Variables|/Game/Geoff_migrated_assets/Garage_stuff/BP_gameinstance_mats.BP_gameinstance_mats_C|Getnumber_laps_selected _asbp_gameinstance_mats_2))
  (bind _returnvalue (Actor|GetActorOfClass "/Game/Geoff_migrated_assets/car_meshes/AI_Car/BP_ai_spline_car4.BP_ai_spline_car4_C"))
  (Variables|Default|Setspline2%20ref _returnvalue)
  (Audio|Components|Audio|Stop (Variables|Default|GetSkeletalMesh))
  (Utilities|FlowControl|Delay 4.0)
  (Variables|Default|Setrace%20just%20started? false)
  (Components|Animation|PlayAnimation (Variables|Default|GetSkeletalMesh) "/Game/Geoff_migrated_assets/car_meshes/AI_Car/Delorean_animated/delorean_straight_line_anim_Anim.delorean_straight_line_anim_Anim" true)
  (CallFunction|MoveAiCar)
  (Utilities|FlowControl|Delay 3.0 :!label _label)
  (CallFunction|ChangeAICarSpeed)
  (goto _label))

(event Game|Damage|EventAnyDamage
  (params (Damage :type Float%20%28single-precision%29) (DamageType :type Damage%20Type%20Object%20Reference) (InstigatedBy :type Controller%20Object%20Reference) (DamageCauser :type Actor%20Object%20Reference))
  ;[1 1 1] damage to hitpoints
  (Variables|Default|SetAI_car2_hitpoints (Math|Float|Clamp(Float) (- (Variables|Default|GetAI_car2_hitpoints) Damage) 0.0 (Variables|Default|GetAI_car2_maxhitpoints))))

(event EventTick
  (params (DeltaSeconds :type Float%20%28single-precision%29))
  (bind _returnvalue (Transformation|GetActorRotation))
  (bind _front_pitch_trace_start (Variables|Default|Getfront%20pitch%20trace%20start))
  (bind _height_trace_start (Variables|Default|Getheight%20trace%20start))
  (bind _rear_pitch_trace_start (Variables|Default|Getrear%20pitch%20trace%20start))
  (bind _right_roll_trace_start1 (Variables|Default|Getright%20roll%20trace%20start1))
  (bind _left_roll_trace_start2 (Variables|Default|Getleft%20roll%20trace%20start2))
  (bind _returnvalue_2 (Transformation|GetWorldLocation _front_pitch_trace_start))
  (bind _returnvalue_3 (Transformation|GetWorldLocation _rear_pitch_trace_start))
  (bind _returnvalue_4 (Transformation|GetWorldLocation _height_trace_start))
  (bind _returnvalue_5 (Transformation|GetWorldLocation _right_roll_trace_start1))
  (bind _returnvalue_6 (Transformation|GetWorldLocation _left_roll_trace_start2))
  (if (Variables|Default|Getelimination%20race?)
    (bind _asavs_game_mode (Utilities|Casting|CastToAVS_GameMode (Game|GetGameMode)))
    (if (Variables|/Game/AVS/AVS_GameMode.AVS_GameMode_C|GetAI%20car%203%20eliminated? _asavs_game_mode)
      (Actor|DestroyActor)
      (else
        (bind _asavs_game_mode_2 (Utilities|Casting|CastToAVS_GameMode (Game|GetGameMode) :!label _label))
        (Variables|/Game/AVS/AVS_GameMode.AVS_GameMode_C|Setai_car_3_location _asavs_game_mode_2 (Transformation|GetWorldTransform (Variables|Default|GetSkeletalMesh)))
        (if (not (Variables|Default|Getrace%20just%20started?))
          (CallFunction|WeaponTrace)
          (CallFunction|CollisionTrace)
          (if (Variables|Default|Getavoiding%20collision?)
            (Utilities|FlowControl|Delay 1.0)
            (Variables|Default|Setavoiding%20collision? false)
            (Audio|Components|Audio|Play (Variables|Default|Getmove%20ai%20car)))
          (if (<= (Variables|Default|GetAI_car2_hitpoints) 0.0)
            ;[1 1 1] death pause
            (if (Variables|Default|Getelimination%20race?)
              (Actor|DestroyActor)
              (bind _asavs_game_mode_3 (Utilities|Casting|CastToAVS_GameMode (Game|GetGameMode)))
              (Variables|/Game/AVS/AVS_GameMode.AVS_GameMode_C|Setai_car_3_checkpoints%20passed _asavs_game_mode_3 0)
              (Variables|/Game/AVS/AVS_GameMode.AVS_GameMode_C|SetAI%20car%201%20eliminated? _asavs_game_mode_3 true)
              (Variables|/Game/AVS/AVS_GameMode.AVS_GameMode_C|Setnumber%20of%20players%20eliminated _asavs_game_mode_3 (+ (Variables|/Game/AVS/AVS_GameMode.AVS_GameMode_C|Getnumber%20of%20players%20eliminated _asavs_game_mode_3) 1))
              (else
                (Audio|Components|Audio|Stop (Variables|Default|GetSkeletalMesh))
                (if (Variables|Default|Gettimeline%20stopped?)
                  (Rendering|ToggleVisibility (Variables|Default|GetScene) true :!label _label_2)
                  (if (> (Variables|Default|Getai%20respawn%20flash%20timer) 3.0)
                    (Variables|Default|SetAI_car2_hitpoints (Variables|Default|GetAI_car2_maxhitpoints))
                    (Variables|Default|Setai%20respawn%20flash%20timer 0.0)
                    (Variables|Default|Settimeline%20stopped? false)
                    (Utilities|FlowControl|Delay 4.0)
                    (Rendering|SetVisibility (Variables|Default|GetScene) true true)
                    (Components|Animation|PlayAnimation (Variables|Default|GetSkeletalMesh) "/Game/Geoff_migrated_assets/car_meshes/AI_Car/Delorean_animated/delorean_straight_line_anim_Anim.delorean_straight_line_anim_Anim" true)
                    (bind _newtrack_0 (Timeline|move%20ai%20car Play)
                      (:Update
                        (bind _outhit (Collision|LineTraceByChannel _returnvalue_4 (+ _returnvalue_4 (* (Math|Vector|GetForwardVector (Transformation|GetWorldRotation _height_trace_start)) 1e+03)) "TraceTypeQuery1" false 0 "None"))
                        (bind _outhit_2 (Collision|LineTraceByChannel _returnvalue_5 (+ _returnvalue_5 (* (Math|Vector|GetForwardVector (Transformation|GetWorldRotation _right_roll_trace_start1)) 1e+03)) "TraceTypeQuery1" false 0 "None"))
                        (bind _outhit_3 (Collision|LineTraceByChannel _returnvalue_6 (+ _returnvalue_6 (* (Math|Vector|GetForwardVector (Transformation|GetWorldRotation _left_roll_trace_start2)) 1e+03)) "TraceTypeQuery1" false 0 "None"))
                        (bind _outhit_4 (Collision|LineTraceByChannel _returnvalue_2 (+ _returnvalue_2 (* (Math|Vector|GetForwardVector (Transformation|GetWorldRotation _front_pitch_trace_start)) 1e+03)) "TraceTypeQuery1" false 0 "None"))
                        (bind _outhit_5 (Collision|LineTraceByChannel _returnvalue_3 (+ _returnvalue_3 (* (Math|Vector|GetForwardVector (Transformation|GetWorldRotation _rear_pitch_trace_start)) 1e+03)) "TraceTypeQuery1" false 0 "None"))
                        (if (< (.Distance (Collision|BreakHitResult _outhit_4)) (.Distance (Collision|BreakHitResult _outhit_5)))
                          (Variables|Default|SetReturn%20Value%20Y%20%28Pitch%29 (+ (.pitch _returnvalue) 0.1))
                          (else
                            (Variables|Default|SetReturn%20Value%20Y%20%28Pitch%29 (- (.pitch _returnvalue) 0.1))))
                        (Transformation|SetActorTransform (Math|Transform|MakeTransform (Math|Vector|MakeVector (.x (Spline|GetLocationatDistanceAlongSpline (Variables|/Game/Geoff_migrated_assets/car_meshes/AI_Car/BP_ai_spline_car4.BP_ai_spline_car4_C|GetSpline (Variables|Default|Getspline2%20ref)) (Math|Float|Lerp 0.0 (Spline|GetSplineLength (Variables|/Game/Geoff_migrated_assets/car_meshes/AI_Car/BP_ai_spline_car4.BP_ai_spline_car4_C|GetSpline (Variables|Default|Getspline2%20ref))) _newtrack_0) "World")) (.y (Spline|GetLocationatDistanceAlongSpline (Variables|/Game/Geoff_migrated_assets/car_meshes/AI_Car/BP_ai_spline_car4.BP_ai_spline_car4_C|GetSpline (Variables|Default|Getspline2%20ref)) (Math|Float|Lerp 0.0 (Spline|GetSplineLength (Variables|/Game/Geoff_migrated_assets/car_meshes/AI_Car/BP_ai_spline_car4.BP_ai_spline_car4_C|GetSpline (Variables|Default|Getspline2%20ref))) _newtrack_0) "World")) (+ (- (.z (Transformation|GetActorLocation)) (.Distance (Collision|BreakHitResult _outhit))) 125.0)) (Math|Rotator|MakeRotator (Variables|Default|GetReturn%20Value%20X%20%28Roll%29) (Variables|Default|GetReturn%20Value%20Y%20%28Pitch%29) (.yaw (Spline|GetRotationatDistanceAlongSpline (Variables|/Game/Geoff_migrated_assets/car_meshes/AI_Car/BP_ai_spline_car4.BP_ai_spline_car4_C|GetSpline (Variables|Default|Getspline2%20ref)) (Math|Float|Lerp 0.0 (Spline|GetSplineLength (Variables|/Game/Geoff_migrated_assets/car_meshes/AI_Car/BP_ai_spline_car4.BP_ai_spline_car4_C|GetSpline (Variables|Default|Getspline2%20ref))) _newtrack_0) "World"))) "1,1,1"))))
                    (else
                      (Variables|Default|Setai%20respawn%20flash%20timer (+ (Variables|Default|Getai%20respawn%20flash%20timer) 0.5))
                      (Utilities|FlowControl|Delay 0.5)
                      (goto _label_2)))
                  (else
                    (Variables|Default|Settimeline%20stopped? true)
                    (Timeline|move%20ai%20car Stop)))))
            (else
              ;[1 1 1] land mine drop experiment
              (CallFunction|VisibleDamageAicar2)
              (Utilities|FlowControl|Delay (* (Math|Random|RandomFloat) 5e+01))
              (bind _returnvalue_7 (Game|SpawnActorfromClass "/Game/Weapons_etc/land_mine/BP_landmine.BP_landmine_C" (Transformation|GetWorldTransform (Variables|Default|Getmine_drop_arrow)) "Undefined" 0 0))
              (Actor|SetLifeSpan _returnvalue_7 3e+01))))))
    (else
      (goto _label))))

(event Collision|EventActorBeginOverlap
  (params (OtherActor :type Actor%20Object%20Reference))
  ;[1 1 1] ai car overlap ai car events - currently disabled awaiting better solution
)

(fn ConstructionScript)

(fn WeaponTrace
  (bind _ai_car_4_gunfire (Variables|Default|Getai%20car%204%20gunfire))
  (bind _returnvalue (Transformation|GetWorldLocation _ai_car_4_gunfire))
  (bind (_outhit _returnvalue_2) (Collision|LineTraceByChannel _returnvalue (+ _returnvalue (* (Math|Vector|GetForwardVector (Transformation|GetWorldRotation _ai_car_4_gunfire)) 8e+03)) "TraceTypeQuery1" false 0 "None"))
  (Game|Damage|ApplyDamage (.HitActor (Collision|BreakHitResult _outhit)) 0.2 0 0)
  (if _returnvalue_2
    (Rendering|SetVisibility (Variables|Default|GetParticleSystem) true false)
    (Effects|SpawnEmitteratLocation "/Game/Effects/Weapons/Impacts/P_AssaultRifle_IH.P_AssaultRifle_IH" (.Location (Collision|BreakHitResult _outhit)))
    (else
      (Rendering|SetVisibility (Variables|Default|GetParticleSystem) false false))))

(fn CollisionTrace
  (bind _collision_trace (Variables|Default|Getcollision%20trace))
  (bind _returnvalue (Transformation|GetWorldLocation _collision_trace))
  (if (not (Variables|Default|Getrace%20just%20started?))
    (bind _outhit (Collision|LineTraceByChannel _returnvalue (+ _returnvalue (* (Math|Vector|GetForwardVector (Transformation|GetWorldRotation _collision_trace)) 5e+02)) "TraceTypeQuery1" false 0 "None"))
    (Utilities|Casting|CastToBP_ai_car_3 (.hitactor _outhit)
      (:then
        _)
      (:CastFailed
        (Utilities|Casting|CastToBP_ai_car_2 (.hitactor _outhit))))
    (Audio|Components|Audio|Stop (Variables|Default|Getmove%20ai%20car))
    (Variables|Default|Setavoiding%20collision? true)))