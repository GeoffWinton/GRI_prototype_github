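; AI race car that follows the BP_ai_spline_car2 spline after a four-second start delay, taking damage and dropping landmines.
; A timeline sets position and yaw along the spline, while downward-offset line traces adjust height and nudge pitch; trace-based roll logic is disconnected.
; Tick spawns mines after random delays and reveals fire and smoke as hitpoints fall.
; Lap count is read from the game instance but unused here.
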(event Custom|visible%20damage_aicar2
  ;[1 1 1] damage visibility
  (if (< (/ (Variables|Default|GetAI_car2_hitpoints) (Variables|Default|GetAI_car2_maxhitpoints)) 0.75)
    (Rendering|SetVisibility (Variables|Default|Getai_car2_front_fire) true false)
    (if (< (/ (Variables|Default|GetAI_car2_hitpoints) (Variables|Default|GetAI_car2_maxhitpoints)) 0.5)
      (Rendering|SetVisibility (Variables|Default|Getai_car2_rear_fire) true false)
      (if (< (/ (Variables|Default|GetAI_car2_hitpoints) (Variables|Default|GetAI_car2_maxhitpoints)) 0.25)
        (Rendering|SetVisibility (Variables|Default|Getai_car_2_smoke) true false)))))

(event Custom|move%20ai%20car
  (bind _returnvalue (Transformation|GetActorRotation))
  (bind _front_pitch_trace_start (Variables|Default|Getfront%20pitch%20trace%20start))
  (bind _height_trace_start (Variables|Default|Getheight%20trace%20start))
  (bind _rear_pitch_trace_start (Variables|Default|Getrear%20pitch%20trace%20start))
  (bind _right_roll_trace_start1 (Variables|Default|Getright%20roll%20trace%20start1))
  (bind _left_roll_trace_start2 (Variables|Default|Getleft%20roll%20trace%20start2))
  (bind _returnvalue_2 (Transformation|GetWorldLocation _front_pitch_trace_start))
  (bind _returnvalue_3 (Transformation|GetWorldLocation _rear_pitch_trace_start))
  (bind _returnvalue_4 (Transformation|GetWorldLocation _height_trace_start))
  (bind _returnvalue_5 (Transformation|GetWorldLocation _right_roll_trace_start1))
  (bind _returnvalue_6 (Transformation|GetWorldLocation _left_roll_trace_start2))
  (Components|Timeline|SetPlayRate (Variables|Default|Getmove%20ai%20car) (/ 1.0 (Variables|Default|Gettime%20to%20complete%20%28seconds%29)))
  (bind _newtrack_0 (Timeline|move%20ai%20car Play)
    (:Update
      (bind _outhit (Collision|LineTraceByChannel _returnvalue_4 (+ _returnvalue_4 (* (Math|Vector|GetForwardVector (Transformation|GetWorldRotation _height_trace_start)) 1e+03)) "TraceTypeQuery1" false 0 "None"))
      (bind _outhit_2 (Collision|LineTraceByChannel _returnvalue_5 (+ _returnvalue_5 (* (Math|Vector|GetForwardVector (Transformation|GetWorldRotation _right_roll_trace_start1)) 1e+03)) "TraceTypeQuery1" false 0 "None"))
      (bind _outhit_3 (Collision|LineTraceByChannel _returnvalue_6 (+ _returnvalue_6 (* (Math|Vector|GetForwardVector (Transformation|GetWorldRotation _left_roll_trace_start2)) 1e+03)) "TraceTypeQuery1" false 0 "None"))
      (bind _outhit_4 (Collision|LineTraceByChannel _returnvalue_2 (+ _returnvalue_2 (* (Math|Vector|GetForwardVector (Transformation|GetWorldRotation _front_pitch_trace_start)) 1e+03)) "TraceTypeQuery1" false 0 "None"))
      (bind _outhit_5 (Collision|LineTraceByChannel _returnvalue_3 (+ _returnvalue_3 (* (Math|Vector|GetForwardVector (Transformation|GetWorldRotation _rear_pitch_trace_start)) 1e+03)) "TraceTypeQuery1" false 0 "None"))
      (if (< (.Distance (Collision|BreakHitResult _outhit_4)) (.Distance (Collision|BreakHitResult _outhit_5)))
        (Variables|Default|SetReturn%20Value%20Y%20%28Pitch%29 (+ (.pitch _returnvalue) 0.1))
        (else
          (Variables|Default|SetReturn%20Value%20Y%20%28Pitch%29 (- (.pitch _returnvalue) 0.1))))
      (Transformation|SetActorTransform (Math|Transform|MakeTransform (Math|Vector|MakeVector (.x (Spline|GetLocationatDistanceAlongSpline (Variables|/Game/Geoff_migrated_assets/car_meshes/AI_Car/BP_ai_spline_car2.BP_ai_spline_car2_C|Getspline (Variables|Default|Getspline2%20ref)) (Math|Float|Lerp 0.0 (Spline|GetSplineLength (Variables|/Game/Geoff_migrated_assets/car_meshes/AI_Car/BP_ai_spline_car2.BP_ai_spline_car2_C|Getspline (Variables|Default|Getspline2%20ref))) _newtrack_0) "World")) (.y (Spline|GetLocationatDistanceAlongSpline (Variables|/Game/Geoff_migrated_assets/car_meshes/AI_Car/BP_ai_spline_car2.BP_ai_spline_car2_C|Getspline (Variables|Default|Getspline2%20ref)) (Math|Float|Lerp 0.0 (Spline|GetSplineLength (Variables|/Game/Geoff_migrated_assets/car_meshes/AI_Car/BP_ai_spline_car2.BP_ai_spline_car2_C|Getspline (Variables|Default|Getspline2%20ref))) _newtrack_0) "World")) (+ (- (.z (Transformation|GetActorLocation)) (.Distance (Collision|BreakHitResult _outhit))) 125.0)) (Math|Rotator|MakeRotator (Variables|Default|GetReturn%20Value%20X%20%28Roll%29) (Variables|Default|GetReturn%20Value%20Y%20%28Pitch%29) (.yaw (Spline|GetRotationatDistanceAlongSpline (Variables|/Game/Geoff_migrated_assets/car_meshes/AI_Car/BP_ai_spline_car2.BP_ai_spline_car2_C|Getspline (Variables|Default|Getspline2%20ref)) (Math|Float|Lerp 0.0 (Spline|GetSplineLength (Variables|/Game/Geoff_migrated_assets/car_meshes/AI_Car/BP_ai_spline_car2.BP_ai_spline_car2_C|Getspline (Variables|Default|Getspline2%20ref))) _newtrack_0) "World"))) "1,1,1")))))

(event EventBeginPlay
  (bind _asbp_gameinstance_mats (Utilities|Casting|CastToBP_gameinstance_mats (Game|GetGameInstance)))
  (Variables|Default|Setlaps%20left (Variables|/Game/Geoff_migrated_assets/Garage_stuff/BP_gameinstance_mats.BP_gameinstance_mats_C|Getnumber_laps_selected _asbp_gameinstance_mats))
  (bind _returnvalue (Actor|GetActorOfClass "/Game/Geoff_migrated_assets/car_meshes/AI_Car/BP_ai_spline_car2.BP_ai_spline_car2_C"))
  (Variables|Default|Setspline2%20ref _returnvalue)
  (Audio|Components|Audio|Stop (Variables|Default|GetSkeletalMesh))
  (Utilities|FlowControl|Delay 4.0)
  (Components|Animation|PlayAnimation (Variables|Default|GetSkeletalMesh) "/Game/Geoff_migrated_assets/car_meshes/AI_Car/geoff_car_animated/anim1_Anim.anim1_Anim" true)
  (CallFunction|MoveAiCar))

(event Game|Damage|EventAnyDamage
  (params (Damage :type Float%20%28single-precision%29) (DamageType :type Damage%20Type%20Object%20Reference) (InstigatedBy :type Controller%20Object%20Reference) (DamageCauser :type Actor%20Object%20Reference))
  ;[1 1 1] damage to hitpoints
  (Variables|Default|SetAI_car2_hitpoints (Math|Float|Clamp(Float) (- (Variables|Default|GetAI_car2_hitpoints) Damage) 0.0 (Variables|Default|GetAI_car2_maxhitpoints))))

(event EventTick
  (params (DeltaSeconds :type Float%20%28single-precision%29))
  ;[1 1 1] land mine drop experiment
  (CallFunction|VisibleDamageAicar2)
  (Utilities|FlowControl|Delay (* (Math|Random|RandomFloat) 1e+01))
  (Game|SpawnActorfromClass "/Game/Weapons_etc/land_mine/BP_landmine.BP_landmine_C" (Transformation|GetWorldTransform (Variables|Default|Getmine_drop_arrow)) "Undefined" 0 0))

(fn ConstructionScript)