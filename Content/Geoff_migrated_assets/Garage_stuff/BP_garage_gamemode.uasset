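; Game mode for the garage that manages the switch from player-count selection to the main garage UI.
; On BeginPlay it clears all widgets and shows the player choice widget.
; Tick polls a flag for the player-count choice; once set, a DoOnce swaps in the garage widget and starts a Miles Davis music track as 2D sound.
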(event EventBeginPlay
  ;[1 1 1] add player choice widget
  (Viewport|RemoveAllWidgets)
  (bind _returnvalue (UserInterface|CreateWidget "/Game/Geoff_migrated_assets/Garage_stuff/garage_player_choice_widget.garage_player_choice_widget_C"))
  (UserInterface|Viewport|AddtoViewport _returnvalue 0))

(event EventTick
  (params (DeltaSeconds :type Float%20%28single-precision%29))
  ;[1 1 1] add garage widget
  (if (Variables|Default|Getnumber_of_players_choice_made?)
    (Utilities|FlowControl|DoOnce false
      (:Completed
        (Viewport|RemoveAllWidgets)
        (bind _returnvalue (UserInterface|CreateWidget "/Game/Geoff_migrated_assets/Garage_stuff/BP_garage_widget.BP_garage_widget_C"))
        (UserInterface|Viewport|AddtoViewport _returnvalue 0)
        (Audio|PlaySound2D "/Game/Sounds/Miles_Davis_-_Freddie_Freeloader__Official_Audio_.Miles_Davis_-_Freddie_Freeloader__Official_Audio_" 1.0 1.0 0.0 0 0)))))

(fn ConstructionScript)