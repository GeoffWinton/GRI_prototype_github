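; Garage preview car that lets one or two players take turns choosing a vehicle and paint colour.
; Tick polls player 0's garage controller, using DoOnce-gated right-stick input to cycle material or frame/wheelset arrays by menu selection, special-casing Delorean paint.
; An axis input revolves the spring arm around the car.
; Confirming saves choices to the game instance, then hands over to player two via the game mode or fades to the main menu.
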(event EventBeginPlay
  ;[1 1 1] fade in and set variables
  (CameraFades|StartCameraFade :self (Game|GetPlayerCameraManager 0) :FromAlpha 1.0 :Duration 1.0)
  (Utilities|FlowControl|Delay 1.0)
  (Variables|Default|Setcurrent%20rotation (Math|Vector|MakeVector 0.0 0.0 (.yaw (Variables|/Script/Engine.SceneComponent|GetRelativeRotation (Variables|Default|GetSpringArm)))))
  (Variables|Default|Setnumber%20of%20materials (- (Utilities|Array|Length (Variables|Default|Getmaterial_array)) 1))
  (Variables|Default|Setnumber%20of%20frames (- (Utilities|Array|Length (Variables|Default|Getframes%20array)) 1)))

(event EventTick
  (params (DeltaSeconds :type Float%20%28single-precision%29))
  ;[1 1 1] material selection
  (bind _asgarage_controller (Utilities|Casting|CastTogarage_controller (Game|GetPlayerController 0)))
  (if (Variables|Default|Getplayer1_choosing?)
    (if (> (Variables|/Game/Geoff_migrated_assets/Garage_stuff/garage_controller.garage_controller_C|Getright_stick_value _asgarage_controller) 0.0)
      (Utilities|FlowControl|DoOnce false :!label _label
        (:Completed
          (bind _asgarage_controller_2 (Utilities|Casting|CastTogarage_controller (Game|GetPlayerController 0)))
          (if (Utilities|Name|Equal(Name) (Variables|/Game/Geoff_migrated_assets/Garage_stuff/garage_controller.garage_controller_C|Getgarage_men_selection_name _asgarage_controller_2) "choose_colour")
            (if (< (Variables|Default|Getarray_position_mats) (Variables|Default|Getnumber%20of%20materials))
              (Variables|Default|Setarray_position_mats (+ (Variables|Default|Getarray_position_mats) 1))
              (else
                (Variables|Default|Setarray_position_mats 0)))
            (Variables|Default|Setnew%20material (Utilities|Array|Get(acopy) (Variables|Default|Getmaterial_array) (Variables|Default|Getarray_position_mats)))
            (if (Utilities|Name|Equal(Name) (Utilities|Array|Get(acopy) (Variables|Default|Getcar_selection_names) (Variables|Default|Getarray_position_frames)) "Delorean")
              (Rendering|Material|SetMaterial (Variables|Default|Getframe) 1 (Variables|Default|Getnew%20material))
              (Rendering|Material|SetMaterial (Variables|Default|Getframe) 0 (Utilities|Array|Get(acopy) (Variables|Default|Getmaterial_array) 5))
              (else
                (Rendering|Material|SetMaterial (Variables|Default|Getframe) 0 (Variables|Default|Getnew%20material))))
            (Utilities|FlowControl|Delay 0.2)
            (else
              ;[1 1 1] choose frame
              (bind _asgarage_controller_3 (Utilities|Casting|CastTogarage_controller (Game|GetPlayerController 0) :!label _label_2))
              (if (Variables|Default|Getplayer1_choosing?)
                (if (> (Variables|/Game/Geoff_migrated_assets/Garage_stuff/garage_controller.garage_controller_C|Getright_stick_value _asgarage_controller_3) 0.0)
                  (Development|PrintString "Hello")
                  (Utilities|FlowControl|DoOnce false :!label _label_3
                    (:Completed
                      (bind _asgarage_controller_4 (Utilities|Casting|CastTogarage_controller (Game|GetPlayerController 0)))
                      (if (Utilities|Name|Equal(Name) (Variables|/Game/Geoff_migrated_assets/Garage_stuff/garage_controller.garage_controller_C|Getgarage_men_selection_name _asgarage_controller_4) "choose_car")
                        (Rendering|Material|SetMaterial (Variables|Default|Getframe) 0 (Utilities|Array|Get(acopy) (Variables|Default|Getelement0_defaults) (+ (Variables|Default|Getarray_position_frames) 1)))
                        (Rendering|Material|SetMaterial (Variables|Default|Getframe) 1 (Utilities|Array|Get(acopy) (Variables|Default|Getelement1_defaults) (+ (Variables|Default|Getarray_position_frames) 1)))
                        (if (< (Variables|Default|Getarray_position_frames) (Variables|Default|Getnumber%20of%20frames))
                          (Variables|Default|Setarray_position_frames (+ (Variables|Default|Getarray_position_frames) 1))
                          (else
                            (Variables|Default|Setarray_position_frames 0)))
                        (Components|StaticMesh|SetStaticMesh (Variables|Default|Getframe) (Utilities|Array|Get(acopy) (Variables|Default|Getframes%20array) (Variables|Default|Getarray_position_frames)))
                        (Components|StaticMesh|SetStaticMesh (Variables|Default|Getwheelset) (Utilities|Array|Get(acopy) (Variables|Default|Getwheelsets%20array) (Variables|Default|Getarray_position_frames)))
                        (Transformation|SetRelativeTransform (Variables|Default|Getwheelset) (Utilities|Array|Get(acopy) (Variables|Default|Getwheelsets_transform_array) (Variables|Default|Getarray_position_frames)) false false)
                        (Transformation|SetRelativeTransform (Variables|Default|Getframe) (Utilities|Array|Get(acopy) (Variables|Default|Getframe_transform_array) (Variables|Default|Getarray_position_frames)) false false)
                        (Variables|Default|Setcar_chosen_name (Utilities|Array|Get(acopy) (Variables|Default|Getcar_selection_names) (Variables|Default|Getarray_position_frames)))
                        (goto _label_3 Reset))))
                  (else
                    (goto _label_3 Reset)))
                (elif (Variables|Default|Getplayer2_choosing?)
                  (if (> (Variables|/Game/Geoff_migrated_assets/Garage_stuff/garage_controller.garage_controller_C|Getright_stick_value _asgarage_controller_3) 0.0)
                    (Utilities|FlowControl|DoOnce false :!label _label_4
                      (:Completed
                        (bind _asgarage_controller_5 (Utilities|Casting|CastTogarage_controller (Game|GetPlayerController 0)))
                        (if (Utilities|Name|Equal(Name) (Variables|/Game/Geoff_migrated_assets/Garage_stuff/garage_controller.garage_controller_C|Getgarage_men_selection_name _asgarage_controller_5) "choose_car")
                          (Rendering|Material|SetMaterial (Variables|Default|Getframe) 0 (Utilities|Array|Get(acopy) (Variables|Default|Getelement0_defaults) (+ (Variables|Default|Getarray_position_frames) 1)))
                          (Rendering|Material|SetMaterial (Variables|Default|Getframe) 1 (Utilities|Array|Get(acopy) (Variables|Default|Getelement1_defaults) (+ (Variables|Default|Getarray_position_frames) 1)))
                          (if (< (Variables|Default|Getarray_position_frames) (Variables|Default|Getnumber%20of%20frames))
                            (Variables|Default|Setarray_position_frames (+ (Variables|Default|Getarray_position_frames) 1))
                            (else
                              (Variables|Default|Setarray_position_frames 0)))
                          (Components|StaticMesh|SetStaticMesh (Variables|Default|Getframe) (Utilities|Array|Get(acopy) (Variables|Default|Getframes%20array) (Variables|Default|Getarray_position_frames)))
                          (Components|StaticMesh|SetStaticMesh (Variables|Default|Getwheelset) (Utilities|Array|Get(acopy) (Variables|Default|Getwheelsets%20array) (Variables|Default|Getarray_position_frames)))
                          (Transformation|SetRelativeTransform (Variables|Default|Getwheelset) (Utilities|Array|Get(acopy) (Variables|Default|Getwheelsets_transform_array) (Variables|Default|Getarray_position_frames)) false false)
                          (Transformation|SetRelativeTransform (Variables|Default|Getframe) (Utilities|Array|Get(acopy) (Variables|Default|Getframe_transform_array) (Variables|Default|Getarray_position_frames)) false false)
                          (Variables|Default|Setcar_chosen_name (Utilities|Array|Get(acopy) (Variables|Default|Getcar_selection_names) (Variables|Default|Getarray_position_frames)))
                          (Utilities|FlowControl|Delay 0.2)
                          (goto _label_4 Reset))))
                    (else
                      (goto _label_4 Reset)))))))))
      (else
        (goto _label Reset)))
    (elif (Variables|Default|Getplayer2_choosing?)
      (if (> (Variables|/Game/Geoff_migrated_assets/Garage_stuff/garage_controller.garage_controller_C|Getright_stick_value _asgarage_controller) 0.0)
        (Utilities|FlowControl|DoOnce false :!label _label_5
          (:Completed
            (bind _asgarage_controller_6 (Utilities|Casting|CastTogarage_controller (Game|GetPlayerController 0)))
            (if (Utilities|Name|Equal(Name) (Variables|/Game/Geoff_migrated_assets/Garage_stuff/garage_controller.garage_controller_C|Getgarage_men_selection_name _asgarage_controller_6) "choose_colour")
              (if (< (Variables|Default|Getarray_position_mats) (Variables|Default|Getnumber%20of%20materials))
                (Variables|Default|Setarray_position_mats (+ (Variables|Default|Getarray_position_mats) 1))
                (else
                  (Variables|Default|Setarray_position_mats 0)))
              (Variables|Default|Setnew%20material (Utilities|Array|Get(acopy) (Variables|Default|Getmaterial_array) (Variables|Default|Getarray_position_mats)))
              (if (Utilities|Name|Equal(Name) (Utilities|Array|Get(acopy) (Variables|Default|Getcar_selection_names) (Variables|Default|Getarray_position_frames)) "Delorean")
                (Rendering|Material|SetMaterial (Variables|Default|Getframe) 1 (Variables|Default|Getnew%20material))
                (Rendering|Material|SetMaterial (Variables|Default|Getframe) 0 (Utilities|Array|Get(acopy) (Variables|Default|Getmaterial_array) 5))
                (else
                  (Rendering|Material|SetMaterial (Variables|Default|Getframe) 0 (Variables|Default|Getnew%20material))))
              (Utilities|FlowControl|Delay 0.2)
              (else
                (goto _label_2)))))
        (else
          (goto _label_5 Reset))))))

(event Input|ActionEvents|InputActionchoosematerial
  (params (Key :type Key%20Structure :default "None"))
  ;[1 1 1] choose material and exit
  (:Pressed
    (if (Variables|Default|Getplayer1_choosing?)
      (bind _asbp_gameinstance_mats (Utilities|Casting|CastToBP_gameinstance_mats (Game|GetGameInstance)))
      (Variables|/Game/Geoff_migrated_assets/Garage_stuff/BP_gameinstance_mats.BP_gameinstance_mats_C|Setplayer1_material_chosen _asbp_gameinstance_mats (Variables|Default|Getnew%20material))
      (Variables|/Game/Geoff_migrated_assets/Garage_stuff/BP_gameinstance_mats.BP_gameinstance_mats_C|Setplayer1car _asbp_gameinstance_mats (Variables|Default|Getcar%20chosen))
      (Variables|/Game/Geoff_migrated_assets/Garage_stuff/BP_gameinstance_mats.BP_gameinstance_mats_C|Setplayer1_car_selection _asbp_gameinstance_mats (Variables|Default|Getcar_chosen_name))
      (bind _asbp_gameinstance_mats_2 (Utilities|Casting|CastToBP_gameinstance_mats (Game|GetGameInstance)))
      (if (== (Variables|/Game/Geoff_migrated_assets/Garage_stuff/BP_gameinstance_mats.BP_gameinstance_mats_C|Getnumber_players_selected _asbp_gameinstance_mats_2) 2)
        (Variables|Default|Setplayer1_choosing? false)
        (Variables|Default|Setplayer2_choosing? true)
        (bind _asbp_garage_gamemode (Utilities|Casting|CastToBP_garage_gamemode (Game|GetGameMode)))
        (Variables|/Game/Geoff_migrated_assets/Garage_stuff/BP_garage_gamemode.BP_garage_gamemode_C|Setplayer1_choosing? _asbp_garage_gamemode false)
        (Variables|/Game/Geoff_migrated_assets/Garage_stuff/BP_garage_gamemode.BP_garage_gamemode_C|Setplayer2_choosing? _asbp_garage_gamemode true)
        (Variables|/Game/Geoff_migrated_assets/Garage_stuff/BP_garage_gamemode.BP_garage_gamemode_C|Setchanging_player? _asbp_garage_gamemode true)
        (Utilities|FlowControl|Delay 3.0)
        (Variables|/Game/Geoff_migrated_assets/Garage_stuff/BP_garage_gamemode.BP_garage_gamemode_C|Setchanging_player? _asbp_garage_gamemode false)
        (else
          (CameraFades|StartCameraFade :self (Game|GetPlayerCameraManager 0) :ToAlpha 1.0 :Duration 2.0 :bHoldWhenFinished true :!label _label)
          (Utilities|FlowControl|Delay 2.0)
          (Game|OpenLevel(byName) "Main_menu_level")))
      (elif (Variables|Default|Getplayer2_choosing?)
        (bind _asbp_gameinstance_mats_3 (Utilities|Casting|CastToBP_gameinstance_mats (Game|GetGameInstance)))
        (Variables|/Game/Geoff_migrated_assets/Garage_stuff/BP_gameinstance_mats.BP_gameinstance_mats_C|Setplayer2_material_chosen _asbp_gameinstance_mats_3 (Variables|Default|Getnew%20material))
        (Variables|/Game/Geoff_migrated_assets/Garage_stuff/BP_gameinstance_mats.BP_gameinstance_mats_C|Setplayer1car _asbp_gameinstance_mats_3 (Variables|Default|Getcar%20chosen))
        (Variables|/Game/Geoff_migrated_assets/Garage_stuff/BP_gameinstance_mats.BP_gameinstance_mats_C|Setplayer2_car_selection _asbp_gameinstance_mats_3 (Variables|Default|Getcar_chosen_name))
        (goto _label)))))

(event Input|AxisEvents|InputAxisrevolve_garage_car
  (params (AxisValue :type Float%20%28single-precision%29))
  ;[1 1 1] revolve vehicle
  (Transformation|SetRelativeRotation (Variables|Default|GetSpringArm) (Math|Rotator|MakeRotator 0.0 0.0 (.z (- (Variables|Default|Getcurrent%20rotation) (* AxisValue 1.0)))) false false)
  (Variables|Default|Setcurrent%20rotation (Math|Vector|MakeVector 0.0 0.0 (.z (- (Variables|Default|Getcurrent%20rotation) (* AxisValue 1.0))))))

(fn ConstructionScript)